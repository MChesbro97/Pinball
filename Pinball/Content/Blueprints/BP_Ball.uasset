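; BP_Ball is a physics ball that is constantly pushed along negative world X while being held down toward the surface beneath it.
; Each Tick adds a frame-time-scaled impulse to the Sphere, then runs a debug-drawn Visibility trace straight down.
; The hit normal's Z component, negated and scaled by StickToTable and frame time, becomes a second, purely vertical impulse.
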(event `self.ReceiveTick`
  (params (DeltaSeconds :type "Float (single-precision)"))
  (bind _returnvalue (`self.K2_GetActorLocation`))
  (`PrimitiveComponent.AddImpulse` (`self.Sphere`) (`KismetMathLibrary.MakeVector` (* DeltaSeconds -2000.0)) "None" false)
  (bind _outhit (`KismetSystemLibrary.LineTraceSingle` :`Start` _returnvalue :`End` (+ _returnvalue (0.0 0.0 -300.0)) :`TraceChannel` "TraceTypeQuery1" :`DrawDebugType` "ForDuration"))
  (`PrimitiveComponent.AddImpulse` (`self.Sphere`) (* (* (`.ImpactNormal` (`GameplayStatics.BreakHitResult` _outhit)) (0.0 0.0 -1.0)) (* (`self.StickToTable`) DeltaSeconds)) "None" false))

(fn `UserConstructionScript`)