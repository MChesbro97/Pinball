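; BP_Launcher is a launcher actor whose Cube snaps between a pulled-back and a released position.
; StartPullBack and Release, triggered from outside this graph, set IsPullingBack, move Cube to hard-coded world locations and print debug text.
; Release applies no launch force.
; Unconnected leftover logic would cache the player controller and initial position and drive a gradual, clamped pull-back through a Launching timeline, but it never runs.
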(event `self.ReceiveBeginPlay`)

(event `InputAction|Launch`
  (params (Key :type "Key Structure")))

(event `StartPullBack`
  (set `self.IsPullingBack` true)
  (`SceneComponent.K2_SetWorldLocation` (`self.Cube`) (5460.0 -6460.0 530.0) false false)
  (`KismetSystemLibrary.PrintString` "Pull back"))

(event `Release`
  (set `self.IsPullingBack` false)
  (`SceneComponent.K2_SetWorldLocation` (`self.Cube`) (5640.0 -6460.0 530.0) false false)
  (`KismetSystemLibrary.PrintString` "Released"))

(fn `UserConstructionScript`)