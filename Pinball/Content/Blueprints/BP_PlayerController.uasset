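; Player controller for a pinball game that handles launcher, flipper and pause input.
; BeginPlay shows the score widget, caches the launcher and sorts every flipper into Left and Right arrays by type.
; Launch starts and releases the launcher, while flipper inputs drive every flipper on their side, only when StopGame is true.
; Pause toggles the pause menu, game pause, input mode and cursor; main menu setup is left unwired.
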(event `SetUp`)

(event `self.ReceiveBeginPlay`
  (bind _returnvalue (`|CreateWidget` "/Game/UI/BP_Score.BP_Score_C"))
  (`UserWidget.AddToViewport` _returnvalue 0)
  (`KismetSystemLibrary.DelayUntilNextTick`)
  (bind _returnvalue_2 (`GameplayStatics.GetActorOfClass` "/Game/Blueprints/BP_Launcher2.BP_Launcher2_C"))
  (set `self.Launcher2` _returnvalue_2)
  (bind _outactors (`GameplayStatics.GetAllActorsOfClass` "/Game/Blueprints/BP_Flipper.BP_Flipper_C"))
  (for _array_element _outactors
    (switch `/Game/Blueprints/FlipperType` (`/Game/Blueprints/BP_Flipper.FlipperType` _array_element)
      (:`NewEnumerator0`
        (`KismetArrayLibrary.Array_Add` (`self.Left`) _array_element)
        (bind _returnvalue_3 (`KismetSystemLibrary.GetObjectName` _array_element))
        (`KismetSystemLibrary.PrintString` (`KismetStringLibrary.Concat_StrStr` "Left: " _returnvalue_3)))
      (:`NewEnumerator1`
        (`KismetArrayLibrary.Array_Add` (`self.Right`) _array_element)
        (`KismetSystemLibrary.PrintString` (`KismetStringLibrary.Concat_StrStr` "Right: " _returnvalue_3))))))

(event `InputAction|SetUp`
  (params (Key :type "Key Structure")))

(event `InputAction|Launch`
  (params (Key :type "Key Structure"))
  (bind _launcher2 (`self.Launcher2`))
  (:`Pressed`
    (`KismetSystemLibrary.PrintString` "Launcher2")
    (`/Game/Blueprints/BP_Launcher2.StartLauncherInterp` _launcher2))
  (:`Released`
    (`/Game/Blueprints/BP_Launcher2.ReleaseBall` _launcher2)))

(event `InputAction|RightFlipper`
  (params (Key :type "Key Structure"))
  (bind _right (`self.Right`))
  (bind _stopgame (`self.StopGame`))
  (:`Pressed`
    (if _stopgame
      (for _array_element _right
        (`/Game/Blueprints/BP_Flipper.ActivateFlipper` _array_element))))
  (:`Released`
    (if _stopgame
      (for _array_element_2 _right
        (`/Game/Blueprints/BP_Flipper.DeactivateFlipper` _array_element_2)))))

(event `InputAction|LeftFlipper`
  (params (Key :type "Key Structure"))
  (bind _stopgame (`self.StopGame`))
  (bind _left (`self.Left`))
  (:`Pressed`
    (if _stopgame
      (for _array_element _left
        (`/Game/Blueprints/BP_Flipper.ActivateFlipper` _array_element))))
  (:`Released`
    (if _stopgame
      (for _array_element_2 _left
        (`/Game/Blueprints/BP_Flipper.DeactivateFlipper` _array_element_2)))))

(event `InputAction|Pause`
  (params (Key :type "Key Structure"))
  (bind _returnvalue (`GameplayStatics.GetPlayerController` 0))
  ;[1 1 1] Pause Menu
  (:`Pressed`
    (if (not (`self.isPauseMenuOpen`))
      (set `self.isPauseMenuOpen` true)
      (bind _returnvalue_2 (`|CreateWidget` "/Game/UI/BP_PauseMenu.BP_PauseMenu_C" _returnvalue))
      (bind _output_get (set `self.PauseMenuWidget` _returnvalue_2))
      (`UserWidget.AddToViewport` _output_get 0)
      (`WidgetBlueprintLibrary.SetInputMode_GameAndUIEx` _returnvalue (`self.PauseMenuWidget`))
      (set `PlayerController.bShowMouseCursor` true (`GameplayStatics.GetPlayerController` 0))
      (`GameplayStatics.SetGamePaused` true)
      (else
        (set `self.isPauseMenuOpen` false)
        (`Widget.RemoveFromParent` (`self.PauseMenuWidget`))
        (`GameplayStatics.SetGamePaused` false)
        (`WidgetBlueprintLibrary.SetInputMode_GameOnly` _returnvalue)
        (set `PlayerController.bShowMouseCursor` false (`GameplayStatics.GetPlayerController` 0))))))

(fn `UserConstructionScript`)