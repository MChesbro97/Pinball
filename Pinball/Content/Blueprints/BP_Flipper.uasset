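; Pinball-style flipper actor that swings its Flipper component between a rest and an activated rotation.
; The construction script uses FlipperType (Left or Right) to pick mirrored start and end rotations, apply the start pose, and negate X scale for the left side.
; ActivateFlipper and DeactivateFlipper events animate it to the end or start rotation with MoveComponentTo over FlipTime.
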(event `self.ReceiveBeginPlay`)

(event `ActivateFlipper`
  (`KismetSystemLibrary.MoveComponentTo` (`self.Flipper`) (0.0 0.0 0.0) (`self.EndRotation`) false false (`self.FlipTime`)))

(event `DeactivateFlipper`
  (`KismetSystemLibrary.MoveComponentTo` (`self.Flipper`) (0.0 0.0 0.0) (`self.StartRotation`) false false (`self.FlipTime`)))

(fn `UserConstructionScript`
  (set `self.StartRotation` (select `/Game/Blueprints/FlipperType` (`self.FlipperType`) :`NewEnumerator0` (struct :`Yaw` 20.0) :`NewEnumerator1` (struct :`Yaw` -20.0) :!type "Rotator Structure"))
  (set `self.EndRotation` (select `/Game/Blueprints/FlipperType` (`self.FlipperType`) :`NewEnumerator0` (struct :`Yaw` -20.0) :`NewEnumerator1` (struct :`Yaw` 20.0) :!type "Rotator Structure"))
  (`SceneComponent.K2_SetRelativeRotation` (`self.Flipper`) (`self.StartRotation`) false false)
  (switch `/Game/Blueprints/FlipperType` (`self.FlipperType`)
    (:`NewEnumerator0`
      (`SceneComponent.SetRelativeScale3D` (`self.Flipper`) (-0.5 0.5 0.5)))
    (:`NewEnumerator1`
      (`SceneComponent.SetRelativeScale3D` (`self.Flipper`) (0.5 0.5 0.5)))))