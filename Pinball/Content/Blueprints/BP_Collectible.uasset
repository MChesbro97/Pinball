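; BP_Collectible is a coin pickup that awards score to player 0 and triggers a replacement spawn.
; It fires when an overlap with its Collider ends, without checking which actor overlapped.
; The handler disables Coin overlap events, adds points on BP_PlayerController, plays a sound, passes its transform to BP_Spawner's SpawnNew, then destroys itself.
; The spawner reference is found at BeginPlay or set through Initialize.
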(event `self.ReceiveBeginPlay`
  (bind _returnvalue (`GameplayStatics.GetActorOfClass` "/Game/Blueprints/BP_Spawner.BP_Spawner_C"))
  (set `self.Spawner` _returnvalue))

(event `self.Collider.OnComponentEndOverlap`
  (params (OverlappedComponent :type "PrimitiveComponent Object Reference") (OtherActor :type "Actor Object Reference") (OtherComp :type "PrimitiveComponent Object Reference") (OtherBodyIndex :type Integer))
  (set `PrimitiveComponent.bGenerateOverlapEvents` false (`self.Coin`))
  (bind _asbp_player_controller (cast `/Game/Blueprints/BP_PlayerController` (`GameplayStatics.GetPlayerController` 0)))
  (set `/Game/Blueprints/BP_PlayerController.Score` (+ (`/Game/Blueprints/BP_PlayerController.Score` _asbp_player_controller) 100) _asbp_player_controller)
  (`GameplayStatics.PlaySound2D` "/Game/Assets/341695__projectsu012__coins-1.341695__projectsu012__coins-1" 1.0 1.0 0.0 null null)
  (`/Game/Blueprints/BP_Spawner.SpawnNew` (`self.Spawner`) (`self.GetTransform`))
  (`self.K2_DestroyActor`))

(fn `Initialize`
  (params (Spawner :type "/Game/Blueprints/BP_Spawner Object Reference"))
  (set `self.Spawner` Spawner))

(fn `UserConstructionScript`)